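; TrailGenerator is a component that leaves a trail of Trail actors behind it as it moves.
; Each Tick it measures the straight-line distance from its world location to LastPosition.
; At 100 units or more it spawns a Trail at its world transform, ignoring collisions and passing on its Color, then updates LastPosition, so spacing depends on movement rather than time.
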(event EventBeginPlay)

(event EventTick
  (params (DeltaSeconds :type Float%20%28single-precision%29))
  (if (>= (Math|Vector|VectorLength (- (Transformation|GetWorldLocation) (Variables|Default|GetLastPosition))) 1e+02)
    (Game|SpawnActorfromClass "/Game/Blueprints/Trail.Trail_C" (Transformation|GetWorldTransform) "AlwaysSpawn" 0 (Variables|Default|GetColor) 0)
    (Variables|Default|SetLastPosition (Transformation|GetWorldLocation))))