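; Hover scene component that pushes a physics-simulated mesh away from the surface beneath it.
; InitComponent stores the mesh and enables physics; each Tick traces a fixed distance straight down in world space with debug drawing.
; On a hit, it applies force along the impact normal at its own location, fading from HoverForce with distance over TraceLength, and sets linear and angular damping.
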(event Custom|InitComponent
  (params (MeshComponent :type Static%20Mesh%20Component%20Object%20Reference))
  ;[1 1 1] Simulate Physics
  (bind _output_get (Variables|Default|SetParentComponent MeshComponent))
  (Physics|SetSimulatePhysics _output_get true))

(event EventTick
  (params (DeltaSeconds :type Float%20%28single-precision%29))
  (bind _returnvalue (Transformation|GetWorldLocation))
  ;[1 1 1] Line Trace
  (bind (_outhit _returnvalue_2) (Collision|LineTraceByChannel _returnvalue (- _returnvalue "0, 0,50.000000") "TraceTypeQuery1" false 0 "ForOneFrame"))
  ;[1 1 1] Hover Function
  (if _returnvalue_2
    ;[1 1 1] Set Damping
    (Class|PrimitiveComponent|AddForceatLocation (Variables|Default|GetParentComponent) (* (.ImpactNormal (Collision|BreakHitResult _outhit)) (Math|Float|Lerp (Variables|Default|GetHoverForce) 0.0 (/ (Math|Vector|VectorLength (- (.Location (Collision|BreakHitResult _outhit)) (Transformation|GetWorldLocation))) (Variables|Default|GetTraceLength)))) (Transformation|GetWorldLocation) "None")
    (Class|PrimitiveComponent|SetLinearDamping (Variables|Default|GetParentComponent) (Variables|Default|GetLinearDamping))
    (Class|PrimitiveComponent|SetAngularDamping (Variables|Default|GetParentComponent) (Variables|Default|GetAngularDamping))))