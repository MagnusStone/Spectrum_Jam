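; HoverCar3 is a physics-driven hover car Blueprint that floats on four HoverComponents initialized at BeginPlay, with a lowered center of mass.
; Each Tick derives RPM from an acceleration curve, gated by forward input and a CarPower comparison, and prints it for debugging.
; Tick also counters sideways velocity with a grip force.
; Forward input applies RPM-scaled thrust, while Right input applies torque scaled by forward velocity plus an idle turn term.
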(event EventBeginPlay
  ;[1 1 1] Initialise Hover Components
  (Default|InitComponent (Variables|Default|GetHoverComponent1) (Variables|Default|GetCarMesh))
  ;[1 1 1] Lower Center of Mass
  (Class|PrimitiveComponent|SetCenterOfMass (Variables|Default|GetCarMesh) "0.000000, 0,-50.000000" "None"))

(event Collision|EventActorBeginOverlap
  (params (OtherActor :type Actor%20Object%20Reference)))

(event EventTick
  (params (DeltaSeconds :type Float%20%28single-precision%29))
  (bind _carmesh (Variables|Default|GetCarMesh))
  (bind _carmesh_2 (Variables|Default|GetCarMesh))
  (bind _returnvalue (Math|Vector|GetRightVector _carmesh))
  (Utilities|FlowControl|Sequence
    (:then_0
      (if (> (stale Input|AxisEvents|InputAxisForward AxisValue) 0.0)
        (Utilities|FlowControl|Sequence
          (:then_0
            (bind _result (Math|Float|IncrementFloat (Variables|Default|GetAccelerationRate))))
          (:then_1
            (if (<= (Variables|Default|GetCarPower) (* (* (Math|Curves|GetFloatValue (Variables|Default|GetAcceleration%20Curve) (Variables|Default|GetRPM)) (Variables|Default|GetAccelerationRate)) (* 1.2e+02 DeltaSeconds)))
              (Variables|Default|SetRPM (* (* (Math|Curves|GetFloatValue (Variables|Default|GetAcceleration%20Curve) (Variables|Default|GetRPM)) (Variables|Default|GetAccelerationRate)) (* 1.2e+02 DeltaSeconds))))))))
    (:then_1
      ;[1 1 1] Grip
      ;;[1 1 1] Multiply Inverted Velocity By Grip And Apply As Force
      (Physics|AddForce (Variables|Default|GetCarMesh) (* _returnvalue (* (* (Math|Vector|DotProduct _returnvalue (Transformation|GetComponentVelocity _carmesh)) -1.0) (Variables|Default|GetGrip))) "None" false)
      ;[1 1 1] Turning
      ;;[1 1 1] Get Forward Velocity
      (bind _output_get (Variables|Default|SetForwardVelocity (Math|Vector|DotProduct (Transformation|GetComponentVelocity _carmesh_2) (Math|Vector|GetForwardVector _carmesh_2)))))
    (:then_2
      (Development|PrintString (Utilities|String|ToString(Float) (Variables|Default|GetRPM))))))

(event Input|AxisEvents|InputAxisRight
  (params (AxisValue :type Float%20%28single-precision%29))
  ;[1 1 1] Turning
  ;;[1 1 1] Apply Torque Based On Player Input and Turn Modifier
  (Class|PrimitiveComponent|AddTorque (Variables|Default|GetCarMesh) (Math|Vector|RotateVector (Math|Vector|MakeVector 0.0 0.0 (* AxisValue (+ (/ (stale EventTick _output_get) (Variables|Default|GetTurningSensitivity)) (Variables|Default|GetIdleTurn)))) (Transformation|GetSocketRotation (Variables|Default|GetCarMesh) "")) "None" true))

(event Input|AxisEvents|InputAxisForward
  (params (AxisValue :type Float%20%28single-precision%29))
  ;[1 1 1] Move Forward
  (Physics|AddForce (Variables|Default|GetCarMesh) (* (* (Math|Vector|GetForwardVector (Variables|Default|GetCarMesh)) (Variables|Default|GetRPM)) AxisValue) "None" false))

(fn ConstructionScript)