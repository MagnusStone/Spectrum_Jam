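; Hover component for a vehicle-style Blueprint that pushes a physics-simulated mesh away from the surface a line trace hits.
; InitComponent stores the supplied mesh and enables its physics.
; Each tick it traces from its location to the negated, scaled up vector, used as a world position without adding that location.
; A hit applies force at the component along the impact normal, fading from HoverForce toward zero with distance over TraceLength.
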(event Custom|InitComponent
  (params (MeshComponent :type Static%20Mesh%20Component%20Object%20Reference))
  (bind _output_get (Variables|Default|SetParentComponent MeshComponent))
  (Physics|SetSimulatePhysics _output_get true))

(event EventBeginPlay
  (Development|PrintText "Hover Component Checking In...")
  (Components|Tick|SetComponentTickEnabled true))

(event EventTick
  (params (DeltaSeconds :type Float%20%28single-precision%29))
  (Development|PrintText "Tick")
  (bind (_outhit _returnvalue) (Collision|LineTraceByChannel (Transformation|GetWorldLocation) (* (Math|Vector|GetUpVector) (* (Variables|Default|GetTraceLength) -1.0)) "TraceTypeQuery1" false 0 "ForOneFrame" false))
  (if _returnvalue
    (Class|PrimitiveComponent|AddForceatLocation (Variables|Default|GetParentComponent) (* (.ImpactNormal (Collision|BreakHitResult _outhit)) (Math|Float|Lerp (Variables|Default|GetHoverForce) 0.0 (/ (Math|Vector|VectorLength (- (.Location (Collision|BreakHitResult _outhit)) (Transformation|GetWorldLocation))) (Variables|Default|GetTraceLength)))) (Transformation|GetWorldLocation) "None")
    (Development|PrintText "Hello")))