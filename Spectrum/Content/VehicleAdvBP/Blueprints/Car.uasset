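; Hover car Blueprint that pushes a physics mesh along its forward direction.
; On BeginPlay it passes CarMesh to four hover components for initialization.
; The MoveForward axis event adds a force of CarPower along the mesh's forward vector, ignoring the axis value, so thrust does not depend on input.
; No steering is present, and the Tick and overlap events are empty.
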(event EventBeginPlay
  (Default|InitComponent (Variables|Default|GetHoverComponent1) (Variables|Default|GetCarMesh)))

(event Collision|EventActorBeginOverlap
  (params (OtherActor :type Actor%20Object%20Reference)))

(event EventTick
  (params (DeltaSeconds :type Float%20%28single-precision%29)))

(event Input|AxisEvents|InputAxisMoveForward
  (params (AxisValue :type Float%20%28single-precision%29))
  (Physics|AddForce (Variables|Default|GetCarMesh) (* (Math|Vector|GetForwardVector (Variables|Default|GetCarMesh)) (Variables|Default|GetCarPower)) "None" false))

(fn ConstructionScript)